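; BP_Crystal is a collectable actor that flies to the player and disappears when the player pawn overlaps it.
; On overlap it stores its location, then a timeline alpha lerps it from that point toward the player's current location, re-read each update so it tracks movement.
; The actor destroys itself when the timeline finishes; no score or inventory change happens here.
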(event EventBeginPlay)

(event Collision|EventActorBeginOverlap
  (params (OtherActor :type Actor%20Object%20Reference))
  (if (== OtherActor (Game|Player|GetPlayerPawn 0))
    (Variables|Default|SetLerpStartLocation (Transformation|GetActorLocation))
    (bind _smoothlerpalpha (Timeline|TL_BlendAlpha Play)
      (:Update
        (Transformation|SetActorLocation (Math|Vector|Lerp(Vector) (Variables|Default|GetLerpStartLocation) (Transformation|GetActorLocation (Game|Player|GetPlayerPawn 0)) _smoothlerpalpha) false false))
      (:Finished
        (Actor|DestroyActor)))))

(fn ConstructionScript)